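; A test actor, apparently for learning, that slides its static mesh back and forth along X and experiments with per-actor input.
; UpdateMove adds a relative offset without sweep, flipping the TurnLeft flag at symmetric X limits.
; BeginPlay sets a timer by function name, though the graph shows no target function.
; R prints debug text and 3 disables player input on the actor, while the EnableInput call is unwired.
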(event EventBeginPlay
  (Utilities|Time|SetTimerbyFunctionName 0 "" 0.0))

(event Input|KeyboardEvents|R
  (params (Key :type Key%20Structure :default "None"))
  ;[1 1 1] 다른 액터에게 인풋주기, 인풋을 준다고 해당 액터에게 제어권이 넘어가는 게 아니라 겹치게 되므로, 항상 사용후 비활성 해주어야 한다.
  (:Pressed
    (Development|PrintString "Pressed R Key" true true "(R=1.000000,G=0.031857,B=0.000000,A=1.000000)"))
  (:Released
    (Development|PrintString "Released R Key" true true "(R=1.000000,G=0.031857,B=0.000000,A=1.000000)")))

(event Input|KeyboardEvents|3
  (params (Key :type Key%20Structure :default "None"))
  ;[1 1 1] 다른 액터에게 인풋주기, 인풋을 준다고 해당 액터에게 제어권이 넘어가는 게 아니라 겹치게 되므로, 항상 사용후 비활성 해주어야 한다.
  (:Pressed
    (Input|DisableInput (Game|GetPlayerController 0))))

(fn ConstructionScript)

(fn UpdateMove
  (if (Variables|Default|GetturnLeft)
    ;[1 1 1] Go Left
    (Transformation|AddRelativeLocation (Variables|Default|GetStaticMesh) (* (Variables|Default|GetDelta%20Location) -1.0) false false)
    (if (>= -1e+03 (.x (Variables|/Script/Engine.SceneComponent|GetRelativeLocation (Variables|Default|GetStaticMesh))))
      (Variables|Default|SetturnLeft false))
    (else
      ;[1 1 1] Go Right
      (Transformation|AddRelativeLocation (Variables|Default|GetStaticMesh) (Variables|Default|GetDelta%20Location) false false)
      (if (>= (.x (Variables|/Script/Engine.SceneComponent|GetRelativeLocation (Variables|Default|GetStaticMesh))) 1e+03)
        (Variables|Default|SetturnLeft true)))))