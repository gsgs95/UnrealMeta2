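; BP_MyPawn is a free-flying pawn with adjustable speed and camera controls.
; Axis inputs rotate MyCameraSceneRoot, offset the actor along that root's forward, right and up vectors without sweep or delta time, and zoom by moving MyCamera locally.
; SpeedUp and SpeedDown step all three speeds within clamped limits.
; BeginPlay adds BP_MyWidget to the viewport; Tick is empty, leaving the elapsed-time printing logic and its helper functions disconnected.
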(event EventBeginPlay
  ;[1 1 1] Begin Play (Create Timer Widget)
  (Development|PrintString (Utilities|GetDisplayName self) false false "(R=1.000000,G=0.961361,B=0.000000,A=1.000000)" 6e+01)
  (bind _returnvalue (UserInterface|CreateWidget "/Game/HelloUnreal/BP_MyWidget.BP_MyWidget_C"))
  (bind _output_get (Variables|Default|SetMyWidgetRef _returnvalue))
  (UserInterface|Viewport|AddtoViewport _output_get 0))

(event EventTick
  (params (DeltaSeconds :type Float%20%28single-precision%29))
  ;[1 1 1] Print Elipsed Time Over Tick
  ;;[1 1 1] 시간합해서 정수화
)

(event Input|ActionEvents|InputActionSpeedUp
  (params (Key :type Key%20Structure :default "None"))
  (bind _speeddelta (Variables|MovementValues|GetSpeedDelta))
  (bind _speedupperlimit (Variables|MovementValues|GetSpeedUpperLimit))
  (bind _speedlowerlimit (Variables|MovementValues|GetSpeedLowerLimit))
  ;[1 1 1] SpeedChange
  (:Pressed
    (Variables|MovementValues|SetForwardSpeed (Math|Float|Clamp(Float) (+ _speeddelta (Variables|MovementValues|GetForwardSpeed)) _speedlowerlimit _speedupperlimit))
    (Variables|MovementValues|SetRightSpeed (Math|Float|Clamp(Float) (+ _speeddelta (Variables|MovementValues|GetRightSpeed)) _speedlowerlimit _speedupperlimit))
    (bind _output_get (Variables|MovementValues|SetUpSpeed (Math|Float|Clamp(Float) (+ _speeddelta (Variables|MovementValues|GetUpSpeed)) _speedlowerlimit _speedupperlimit)))
    (Development|PrintString (Utilities|String|ToString(Float) _output_get))))

(event Input|ActionEvents|InputActionSpeedDown
  (params (Key :type Key%20Structure :default "None"))
  (bind _speeddelta (Variables|MovementValues|GetSpeedDelta))
  (bind _speedupperlimit (Variables|MovementValues|GetSpeedUpperLimit))
  (bind _speedlowerlimit (Variables|MovementValues|GetSpeedLowerLimit))
  ;[1 1 1] SpeedChange
  (:Pressed
    (Variables|MovementValues|SetForwardSpeed (Math|Float|Clamp(Float) (- (Variables|MovementValues|GetForwardSpeed) _speeddelta) _speedlowerlimit _speedupperlimit))
    (Variables|MovementValues|SetRightSpeed (Math|Float|Clamp(Float) (- (Variables|MovementValues|GetRightSpeed) _speeddelta) _speedlowerlimit _speedupperlimit))
    (bind _output_get (Variables|MovementValues|SetUpSpeed (Math|Float|Clamp(Float) (- (Variables|MovementValues|GetUpSpeed) _speeddelta) _speedlowerlimit _speedupperlimit)))
    (Development|PrintString (Utilities|String|ToString(Float) _output_get))))

(event Input|AxisEvents|InputAxisUp
  (params (AxisValue :type Float%20%28single-precision%29))
  ;[1 1 1] Actor Movement
  (Transformation|AddActorWorldOffset (* (Math|Vector|GetUpVector (Variables|Default|GetMyCameraSceneRoot)) (* AxisValue (Variables|MovementValues|GetUpSpeed)))))

(event Input|AxisEvents|InputAxisForward
  (params (AxisValue :type Float%20%28single-precision%29))
  ;[1 1 1] Actor Movement
  (Transformation|AddActorWorldOffset (* (Math|Vector|GetForwardVector (Variables|Default|GetMyCameraSceneRoot)) (* AxisValue (Variables|MovementValues|GetForwardSpeed)))))

(event Input|AxisEvents|InputAxisRight
  (params (AxisValue :type Float%20%28single-precision%29))
  ;[1 1 1] Actor Movement
  (Transformation|AddActorWorldOffset (* (Math|Vector|GetRightVector (Variables|Default|GetMyCameraSceneRoot)) (* AxisValue (Variables|MovementValues|GetRightSpeed)))))

(event Input|AxisEvents|InputAxisLookUp
  (params (AxisValue :type Float%20%28single-precision%29))
  ;[1 1 1] Camera Movement
  (Transformation|AddRelativeRotation (Variables|Default|GetMyCameraSceneRoot) (Math|Rotator|MakeRotator 0.0 (* AxisValue -1.0) 0.0) false false))

(event Input|AxisEvents|InputAxisLookRight
  (params (AxisValue :type Float%20%28single-precision%29))
  ;[1 1 1] Camera Movement
  (Transformation|AddRelativeRotation (Variables|Default|GetMyCameraSceneRoot) (Math|Rotator|MakeRotator 0.0 0.0 AxisValue) false false))

(event Input|AxisEvents|InputAxisZoomOut
  (params (AxisValue :type Float%20%28single-precision%29))
  ;[1 1 1] Camera Zoom In and Out Control
  ;;[1 1 1] 단순화
  (Class|SceneComponent|AddLocalTransform (Variables|Default|GetMyCamera) (Math|Transform|MakeTransform (Math|Vector|MakeVector (* AxisValue 1e+02) 0.0 0.0) "0, 0, 0" "1,1,1") false false))

(fn ConstructionScript)

(fn PrintTime
  (params (Min :type Integer) (Sec :type Integer))
  (if (< (Variables|Default|Getsec) 10)
    (if (< (Variables|Default|Getmin) 10)
      (Development|PrintString (Utilities|String|Append (Variables|Default|Gettimeformat) "0" (Utilities|String|ToString(Integer) (Variables|Default|Getmin)) ":" "0" (Utilities|String|ToString(Integer) (Variables|Default|Getsec))) true true "(R=1.000000,G=1.000000,B=1.000000,A=1.000000)" 1.0)
      (else
        (Development|PrintString (Utilities|String|Append (Variables|Default|Gettimeformat) (Utilities|String|ToString(Integer) (Variables|Default|Getmin)) ":" "0" (Utilities|String|ToString(Integer) (Variables|Default|Getsec))) true true "(R=1.000000,G=1.000000,B=1.000000,A=1.000000)" 1.0)))
    (elif true
      (Development|PrintString (Utilities|String|Append (Variables|Default|Gettimeformat) "0" (Utilities|String|ToString(Integer) (Variables|Default|Getmin)) ":" (Utilities|String|ToString(Integer) (Variables|Default|Getsec))) true true "(R=1.000000,G=1.000000,B=1.000000,A=1.000000)" 1.0)
      (else
        (Development|PrintString (Utilities|String|Append (Variables|Default|Gettimeformat) (Utilities|String|ToString(Integer) (Variables|Default|Getmin)) ":" (Utilities|String|ToString(Integer) (Variables|Default|Getsec))) true true "(R=1.000000,G=1.000000,B=1.000000,A=1.000000)" 1.0)))))

(fn InttoString
  (params (Number :type Integer))
  (LocalVariables|SetNum Number)
  (if (< Number 10)
    (return (Utilities|String|Append "0" (Utilities|String|ToString(Integer) (LocalVariables|GetNum))))
    (else
      (return (Utilities|String|ToString(Integer) (LocalVariables|GetNum))))))

(fn AdvencedPrintTime
  (params (Hour :type Integer) (Min :type Integer) (Sec :type Integer))
  (Development|PrintString (Utilities|String|Append (Variables|Default|Gettimeformat) (Utillity|InttoString Hour) ":" (Utillity|InttoString Min) ":" (Utillity|InttoString Sec)) true true "(R=1.000000,G=1.000000,B=1.000000,A=1.000000)" 1.0))

(fn InttoString00
  (params (Number :type Float%20%28single-precision%29))
  (LocalVariables|SetNum (Math|Float|Floor Number))
  (if (< (LocalVariables|GetNum) 10)
    (return (Utilities|String|Append "0" (Utilities|String|ToString(Integer) (LocalVariables|GetNum))))
    (else
      (return (Utilities|String|ToString(Integer) (LocalVariables|GetNum))))))

(fn ComputeTime
  (params (TotalDeltaSecond :type Float%20%28single-precision%29))
  (bind _output_get (Variables|Default|SetTotalDeltaSecond (+ (* 1 TotalDeltaSecond) (Variables|Default|GetTotalDeltaSecond))))
  (Variables|Default|Setsec (Math|Integer|%(Integer) (Math|Conversions|ToInteger(Byte) (Class|KismetMathLibrary|FTrunc64 _output_get)) 60))
  (Variables|Default|Setmin (Math|Integer|%(Integer) (/ (Math|Conversions|ToInteger(Byte) (Class|KismetMathLibrary|FTrunc64 _output_get)) 60) 60))
  (Variables|Default|SetHour (/ (/ (Math|Conversions|ToInteger(Byte) (Class|KismetMathLibrary|FTrunc64 _output_get)) 60) 60)))