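; BP_MoveLeftRight is an actor that slides its Table component back and forth along the X axis under keyboard control.
; It enables input for player controller 0 on BeginPlay, with B starting the motion and M stopping it.
; A timeline drives the relative X location from its scaled XAxis track.
; On Finished it flips IsMoveRight and loops back to Play or Reverse, creating a continuous ping-pong.
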(event EventBeginPlay
  (Input|EnableInput (Game|GetPlayerController 0)))

(event Input|KeyboardEvents|B
  (params (Key :type Key%20Structure :default "None"))
  (:Pressed
    (if (Variables|Default|GetIsMoveRight) :!label _label
      (bind _x_axis (Timeline|타임라인_0 Play)
        (:Update
          (Transformation|SetRelativeLocation (Variables|Default|GetTable) (Math|Vector|MakeVector (* _x_axis 1e+03) 0.0 0.0) false false))
        (:Finished
          (Variables|Default|SetIsMoveRight (not (Variables|Default|GetIsMoveRight)))
          (goto _label)))
      (else
        (Timeline|타임라인_0 Reverse)))))

(event Input|KeyboardEvents|N
  (params (Key :type Key%20Structure :default "None")))

(event Input|KeyboardEvents|M
  (params (Key :type Key%20Structure :default "None"))
  (:Pressed
    (bind _x_axis (Timeline|타임라인_0 Stop)
      (:Update
        (Transformation|SetRelativeLocation (Variables|Default|GetTable) (Math|Vector|MakeVector (* _x_axis 1e+03) 0.0 0.0) false false))
      (:Finished
        (Variables|Default|SetIsMoveRight (not (Variables|Default|GetIsMoveRight)))
        (if (Variables|Default|GetIsMoveRight)
          (Timeline|타임라인_0 Play)
          (else
            (Timeline|타임라인_0 Reverse)))))))

(fn ConstructionScript)