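; BP_MyBox is a collision trigger box that starts moving and rotating objects when its Cube2 component is overlapped.
; Begin overlap calls Play on every entry in MoveRectRef, RotationBalls and MoveRects, with no filter on the overlapping actor.
; End overlap stops only the MoveRectRef entries; it and hit events print component and actor names to the log only.
; An unconnected delay-loop test remains in the event graph and never runs.
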(event OnComponentBeginOverlap(Cube2)
  (params (OverlappedComponent :type Primitive%20Component%20Object%20Reference) (OtherActor :type Actor%20Object%20Reference) (OtherComp :type Primitive%20Component%20Object%20Reference) (OtherBodyIndex :type Integer) (bFromSweep :type Boolean) (SweepResult :type Hit%20Result%20Structure%20%28by%20ref%29))
  (Utilities|FlowControl|Sequence
    (:then_0
      (for _array_element (Variables|Default|GetMoveRectRef)
        (Default|Play _array_element)))
    (:then_1
      (for _array_element_2 (Variables|Default|GetRotationBalls)
        (Default|Play _array_element_2)))
    (:then_2
      (for _array_element_3 (Variables|Default|GetMoveRects)
        (Default|Play _array_element_3)))))

(event OnComponentEndOverlap(Cube2)
  (params (OverlappedComponent :type Primitive%20Component%20Object%20Reference) (OtherActor :type Actor%20Object%20Reference) (OtherComp :type Primitive%20Component%20Object%20Reference) (OtherBodyIndex :type Integer))
  (Development|PrintString (Utilities|String|Append "  EndOverlap" "  OverlappedComponent : " (Utilities|GetDisplayName OverlappedComponent) "  Other Actor : " (Utilities|GetDisplayName OtherActor) "  Other Comp : " (Utilities|GetDisplayName OtherComp)) false true "(R=0.000000,G=0.660000,B=1.000000,A=1.000000)" 2e+02)
  (for _array_element (Variables|Default|GetMoveRectRef)
    (Default|Stop _array_element)))

(event OnComponentHit(Cube2)
  (params (HitComponent :type Primitive%20Component%20Object%20Reference) (OtherActor :type Actor%20Object%20Reference) (OtherComp :type Primitive%20Component%20Object%20Reference) (NormalImpulse :type Vector :default "0, 0, 0") (Hit :type Hit%20Result%20Structure%20%28by%20ref%29))
  (Development|PrintString (Utilities|String|Append "  <OnComponentHit>" "  OverlappedComponent : " (Utilities|GetDisplayName HitComponent) "  Other Actor : " (Utilities|GetDisplayName OtherActor) "  Other Comp : " (Utilities|GetDisplayName OtherComp)) false true "(R=0.000000,G=0.660000,B=1.000000,A=1.000000)" 2e+02))

(fn ConstructionScript)