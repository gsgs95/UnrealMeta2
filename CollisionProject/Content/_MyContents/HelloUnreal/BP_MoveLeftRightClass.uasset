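; BP_MoveLeftRightClass is a test actor that slides its Pole component along relative X using timelines.
; It enables player input on BeginPlay, so B plays 타임라인_0 from the start and M stops it.
; A custom Play event, not called within this Blueprint, ping-pongs 타임라인_1 by flipping IsMoveRight on Finished.
; The B key's reverse branch is unreachable, and the Box overlap handler is empty.
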(event OnComponentBeginOverlap(Box)
  (params (OverlappedComponent :type Primitive%20Component%20Object%20Reference) (OtherActor :type Actor%20Object%20Reference) (OtherComp :type Primitive%20Component%20Object%20Reference) (OtherBodyIndex :type Integer) (bFromSweep :type Boolean) (SweepResult :type Hit%20Result%20Structure%20%28by%20ref%29)))

(event Custom|Play
  (if (Variables|Default|GetIsMoveRight) :!label _label
    (bind _x_axis (Timeline|타임라인_1 Play)
      (:Update
        (Transformation|SetRelativeLocation (Variables|Default|GetPole) (Math|Vector|MakeVector (* _x_axis 1e+03) 0.0 0.0) false false))
      (:Finished
        (Variables|Default|SetIsMoveRight (not (Variables|Default|GetIsMoveRight)))
        (goto _label)))
    (else
      (Timeline|타임라인_1 Reverse))))

(event EventBeginPlay
  (Input|EnableInput (Game|GetPlayerController 0)))

(event Input|KeyboardEvents|B
  (params (Key :type Key%20Structure :default "None"))
  (:Pressed
    (if true
      (bind _x_axis (Timeline|타임라인_0 PlayFromStart)
        (:Update
          (Transformation|SetRelativeLocation (Variables|Default|GetPole) (Math|Vector|MakeVector (* _x_axis 1e+03) 0.0 0.0) false false)))
      (else
        (Timeline|타임라인_0 Reverse)))))

(event Input|KeyboardEvents|N
  (params (Key :type Key%20Structure :default "None")))

(event Input|KeyboardEvents|M
  (params (Key :type Key%20Structure :default "None"))
  (:Pressed
    (bind _x_axis (Timeline|타임라인_0 Stop)
      (:Update
        (Transformation|SetRelativeLocation (Variables|Default|GetPole) (Math|Vector|MakeVector (* _x_axis 1e+03) 0.0 0.0) false false)))))

(fn ConstructionScript)