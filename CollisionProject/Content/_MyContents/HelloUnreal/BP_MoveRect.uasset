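; BP_MoveRect is an actor that moves its static mesh around a rectangular path in the local X-Z plane.
; Play starts a looping timer on UpdateMove and Stop clears it.
; UpdateMove is a four-state machine on MoveType that steps the mesh by Speed and switches direction past the positive or negative MoveScale bound.
; Disconnected leftovers hold a delayed timer stop and an older left-right ping-pong movement.
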(event Custom|Play
  (Utilities|Time|SetTimerbyFunctionName 0 "UpdateMove" 0.1 true))

(event Custom|Stop
  (Utilities|Time|ClearTimerbyFunctionName 0 "UpdateMove"))

(fn ConstructionScript)

(fn UpdateMove
  (switch Utilities|FlowControl|Switch|SwitchonEN_MoveType (Variables|Default|GetMoveType)
    (:NewEnumerator1
      (if (<= (.x (Variables|/Script/Engine.SceneComponent|GetRelativeLocation (Variables|Default|GetStaticMesh))) (Variables|Default|GetMoveScale))
        (Transformation|AddRelativeLocation (Variables|Default|GetStaticMesh) (* "1.000000, 0, 0" (Variables|Default|GetSpeed)) false false)
        (else
          (Variables|Default|SetMoveType "NewEnumerator0"))))
    (:NewEnumerator0
      (if (<= (.z (Variables|/Script/Engine.SceneComponent|GetRelativeLocation (Variables|Default|GetStaticMesh))) (Variables|Default|GetMoveScale))
        (Transformation|AddRelativeLocation (Variables|Default|GetStaticMesh) (* "0.000000, 0,1.000000" (Variables|Default|GetSpeed)) false false)
        (else
          (Variables|Default|SetMoveType "NewEnumerator3"))))
    (:NewEnumerator3
      (if (>= (.x (Variables|/Script/Engine.SceneComponent|GetRelativeLocation (Variables|Default|GetStaticMesh))) (* (Variables|Default|GetMoveScale) -1.0))
        (Transformation|AddRelativeLocation (Variables|Default|GetStaticMesh) (* "-1.000000, 0, 0" (Variables|Default|GetSpeed)) false false)
        (else
          (Variables|Default|SetMoveType "NewEnumerator2"))))
    (:NewEnumerator2
      (if (>= (.z (Variables|/Script/Engine.SceneComponent|GetRelativeLocation (Variables|Default|GetStaticMesh))) (* (Variables|Default|GetMoveScale) -1.0))
        (Transformation|AddRelativeLocation (Variables|Default|GetStaticMesh) (* "0.000000, 0,-1.000000" (Variables|Default|GetSpeed)) false false)
        (else
          (Variables|Default|SetMoveType "NewEnumerator1"))))))